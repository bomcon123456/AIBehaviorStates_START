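; BP_PatrolPath is an enemy AI patrol path actor that visualizes an array of patrol point actors in the level.
; Its construction script builds a linear, optionally looped spline through their locations and adds index text labels above each.
; ShowPatrol is passed directly as the points' hidden-in-game flag, while the labels are destroyed when it is false.
; The event graph holds no logic.
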(event EventBeginPlay)

(event Collision|EventActorBeginOverlap
  (params (OtherActor :type Actor%20Object%20Reference)))

(event EventTick
  (params (DeltaSeconds :type Float%20%28single-precision%29)))

(fn ConstructionScript
  (bind _spline (Variables|Default|GetSpline))
  (for _array_element (Variables|Setup|GetPatrolPoints)
    (Utilities|Array|Add (LocalVariables|GetLocal_PatrolPointLocations) (Transformation|GetActorLocation _array_element))
    (Rendering|SetActorHiddenInGame _array_element (Variables|Setup|GetbShowPatrol)))
  (Utilities|FlowControl|Sequence
    (:then_0
      (Spline|SetSplinePoints _spline (LocalVariables|GetLocal_PatrolPointLocations) "World" true)
      (Utilities|Array|Resize (LocalVariables|GetLocal_SplinePointIndex) (Spline|GetNumberOfSplinePoints _spline))
      (for (_ _array_index) (LocalVariables|GetLocal_SplinePointIndex)
        (Spline|SetSplinePointType (Variables|Default|GetSpline) _array_index "Linear" true))
      (Spline|SetClosedLoop (Variables|Default|GetSpline) (Variables|Setup|GetbLoop) true)
      (for (_array_element_2 _array_index_2) (LocalVariables|GetLocal_PatrolPointLocations)
        (LocalVariables|SetLocal_TextValue (Utilities|Text|ToText(Integer) _array_index_2))
        (bind _returnvalue (AddComponent|AddTextRenderComponent true (Math|Conversions|ToTransform(Vector) (+ _array_element_2 "0, 0,108.000000"))))
        (Utilities|Array|Add (Variables|Default|GetTextRenderArray) _returnvalue)
        (bind _output_get (LocalVariables|SetLocal_TextRenComp _returnvalue))
        (Rendering|Components|TextRender|SetText _output_get (LocalVariables|GetLocal_TextValue))))
    (:then_1
      (if (not (Variables|Setup|GetbShowPatrol))
        (for _array_element_3 (Variables|Default|GetTextRenderArray)
          (Components|DestroyComponent _array_element_3))))))